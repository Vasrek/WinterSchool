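; BP_MasterWeapon2 is a weapon Blueprint that lets a BP_AdventureMan character detect it as a pickup.
; Entering its PickUpAreaRange sets the character's PickUpWeapon to this weapon and shows WeaponName on the character's pickup widget, if that widget is valid.
; Leaving the range clears PickUpWeapon and hides the pickup info.
; The pickup action itself is not in this graph, and the construction script is empty.
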(event `self.PickUpAreaRange.OnComponentBeginOverlap`
  (params (OverlappedComponent :type "PrimitiveComponent Object Reference") (OtherActor :type "Actor Object Reference") (OtherComp :type "PrimitiveComponent Object Reference") (OtherBodyIndex :type Integer) (bFromSweep :type Boolean) (SweepResult :type "HitResult Structure (by ref)"))
  (bind _asbp_adventure_man (cast `/Game/Blueprints/Player/BP_AdventureMan` OtherActor))
  (set `/Game/Blueprints/Player/BP_AdventureMan.PickUpWeapon` self _asbp_adventure_man)
  (bind _pickupwidgetref (`/Game/Blueprints/Player/BP_AdventureMan.PickUpWidgetRef` _asbp_adventure_man))
  (`/Engine/EditorBlueprintResources/StandardMacros.IsValid` _pickupwidgetref
    (:`Is Valid`
      (`/Game/Blueprints/UI/WBP_PickUpWeapon.DisplayPickupInfo` _pickupwidgetref (`self.Weapon Name`)))))

(event `self.PickUpAreaRange.OnComponentEndOverlap`
  (params (OverlappedComponent :type "PrimitiveComponent Object Reference") (OtherActor :type "Actor Object Reference") (OtherComp :type "PrimitiveComponent Object Reference") (OtherBodyIndex :type Integer))
  (bind _asbp_adventure_man (cast `/Game/Blueprints/Player/BP_AdventureMan` OtherActor))
  (set `/Game/Blueprints/Player/BP_AdventureMan.PickUpWeapon` null _asbp_adventure_man)
  (bind _pickupwidgetref (`/Game/Blueprints/Player/BP_AdventureMan.PickUpWidgetRef` _asbp_adventure_man))
  (`/Engine/EditorBlueprintResources/StandardMacros.IsValid` _pickupwidgetref
    (:`Is Valid`
      (`/Game/Blueprints/UI/WBP_PickUpWeapon.HidePickupInfo` _pickupwidgetref))))

(fn `UserConstructionScript`)