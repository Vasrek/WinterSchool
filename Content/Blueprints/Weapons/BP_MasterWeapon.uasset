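; BP_MasterWeapon is a weapon Blueprint, named as a master class, that handles the pickup prompt when a player is near.
; When a BP_Player overlaps PickupArea, it registers itself as that player's PickUpWeapon and shows WeaponName on the player's pickup widget.
; Ending the overlap clears the reference and hides the text, without checking whether another weapon has since set it.
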(event `self.PickupArea.OnComponentBeginOverlap`
  (params (OverlappedComponent :type "PrimitiveComponent Object Reference") (OtherActor :type "Actor Object Reference") (OtherComp :type "PrimitiveComponent Object Reference") (OtherBodyIndex :type Integer) (bFromSweep :type Boolean) (SweepResult :type "HitResult Structure (by ref)"))
  (bind _asbp_player (cast `/Game/Blueprints/Player/BP_Player` OtherActor))
  (set `/Game/Blueprints/Player/BP_Player.PickUpWeapon` self _asbp_player)
  (bind _pickupwidgetref (`/Game/Blueprints/Player/BP_Player.PickUpWidgetRef` _asbp_player))
  (`/Engine/EditorBlueprintResources/StandardMacros.IsValid` _pickupwidgetref
    (:`Is Valid`
      (`/Game/Blueprints/UI/WBP_PickUpWidget.DisplayPickUpText` _pickupwidgetref (`self.WeaponName`)))))

(event `self.PickupArea.OnComponentEndOverlap`
  (params (OverlappedComponent :type "PrimitiveComponent Object Reference") (OtherActor :type "Actor Object Reference") (OtherComp :type "PrimitiveComponent Object Reference") (OtherBodyIndex :type Integer))
  (bind _asbp_player (cast `/Game/Blueprints/Player/BP_Player` OtherActor))
  (set `/Game/Blueprints/Player/BP_Player.PickUpWeapon` null _asbp_player)
  (bind _pickupwidgetref (`/Game/Blueprints/Player/BP_Player.PickUpWidgetRef` _asbp_player))
  (`/Engine/EditorBlueprintResources/StandardMacros.IsValid` _pickupwidgetref
    (:`Is Valid`
      (`/Game/Blueprints/UI/WBP_PickUpWidget.HidePickUpText` _pickupwidgetref))))

(fn `UserConstructionScript`)