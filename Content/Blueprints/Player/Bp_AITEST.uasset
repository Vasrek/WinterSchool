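; Bp_AITEST is a test AI pawn that chases the player and attacks with a katana.
; While CanAttack is false, Tick issues AI MoveTo; arrival plays a montage, then distance to the PlayerController, not the pawn, resets CanAttack.
; Katana overlap damages BP_AdventureMan, with resettable DoOnce gates throttling attacks and hits.
; Katana collision is disabled at BeginPlay and never re-enabled in these graphs.
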(event `self.ReceiveBeginPlay`
  (`PrimitiveComponent.SetCollisionEnabled` (`self.KatanaCollision`) "NoCollision"))

(event `self.ReceiveTick`
  (params (DeltaSeconds :type "Float (single-precision)"))
  (if (not (`self.CanAttack?`))
    (`|AIMoveTo` self (0.0 0.0 0.0) (`GameplayStatics.GetPlayerCharacter` 0) (`self.CloseAttackRange`) true
      (:`OnSuccess`
        (set `self.CanAttack?` true)
        (`/Engine/EditorBlueprintResources/StandardMacros.DoOnce` false :!label _label
          (:`Completed`
            (`self.PlayAnimMontage` "/Game/Temp/AM_KatanaAttack.AM_KatanaAttack")
            (`KismetSystemLibrary.Delay` 1.0)
            (`self.ResetAnimAttack`)
            (if (<= (`self.GetDistanceTo` (`GameplayStatics.GetPlayerController` 0)) (`self.CloseAttackRange`))
              (set `self.CanAttack?` true)
              (else
                (set `self.CanAttack?` false)))))))))

(event `ResetAnimAttack`
  (goto _label :!via `Reset`))

(event `self.KatanaCollision.OnComponentBeginOverlap`
  (params (OverlappedComponent :type "PrimitiveComponent Object Reference") (OtherActor :type "Actor Object Reference") (OtherComp :type "PrimitiveComponent Object Reference") (OtherBodyIndex :type Integer) (bFromSweep :type Boolean) (SweepResult :type "HitResult Structure (by ref)"))
  (bind _asbp_adventure_man (cast `/Game/Blueprints/Player/BP_AdventureMan` OtherActor))
  (`/Engine/EditorBlueprintResources/StandardMacros.DoOnce` false :!label _label_2
    (:`Completed`
      (`/Game/Blueprints/Player/BP_AdventureMan.GetDamage` _asbp_adventure_man (`self.Damage`))
      (`KismetSystemLibrary.Delay` 0.5)
      (`self.ResetAttackDoOnce`))))

(event `ResetAttackDoOnce`
  (goto _label_2 :!via `Reset`))

(fn `UserConstructionScript`)