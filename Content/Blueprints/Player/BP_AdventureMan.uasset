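; BP_AdventureMan is the player character Blueprint, handling walking, camera look and jumping through Enhanced Input.
; BeginPlay adds the IMC_AdventureMan mapping context to player 0's local player subsystem.
; Movement input follows the forward and right vectors of the control rotation's yaw only, so camera pitch does not affect direction.
; Camera input drives controller yaw and pitch, and the jump action starts and stops the built-in Jump.
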(event `self.ReceiveBeginPlay`
  (bind _returnvalue (`GameplayStatics.GetPlayerController` 0))
  (`/Engine/EditorBlueprintResources/StandardMacros.IsValid` _returnvalue
    (:`Is Valid`
      (`EnhancedInputSubsystemInterface.AddMappingContext` (pcsubsystem `EnhancedInputLocalPlayerSubsystem` _returnvalue) "/Game/Blueprints/InputsAdventureMan/IMC_AdventureMan.IMC_AdventureMan" 0 (struct)))))

(event `EnhancedInput|/Game/Blueprints/InputsAdventureMan/Actions/IA_AdventureMovement`
  (params (ActionValue :type "Vector2D Structure") (ElapsedSeconds :type "Float (double-precision)") (TriggeredSeconds :type "Float (double-precision)") (InputAction :type "InputAction Object Reference" :default "/Game/Blueprints/InputsAdventureMan/Actions/IA_AdventureMovement.IA_AdventureMovement"))
  (bind (_returnvalue_roll _returnvalue_pitch _returnvalue_yaw) (`KismetMathLibrary.BreakRotator` (`self.GetControlRotation`)))
  (:`Triggered`
    (`self.AddMovementInput` (`KismetMathLibrary.GetRightVector` (`KismetMathLibrary.MakeRotator` 0.0 0.0 _returnvalue_yaw)) ActionValue_X)
    (`self.AddMovementInput` (`KismetMathLibrary.GetForwardVector` (`KismetMathLibrary.MakeRotator` 0.0 0.0 _returnvalue_yaw)) ActionValue_Y)))

(event `EnhancedInput|/Game/Blueprints/InputsAdventureMan/Actions/IA_AdventureCamera`
  (params (ActionValue :type "Vector2D Structure") (ElapsedSeconds :type "Float (double-precision)") (TriggeredSeconds :type "Float (double-precision)") (InputAction :type "InputAction Object Reference" :default "/Game/Blueprints/InputsAdventureMan/Actions/IA_AdventureCamera.IA_AdventureCamera"))
  (:`Triggered`
    (`self.AddControllerYawInput` ActionValue_X)
    (`self.AddControllerPitchInput` ActionValue_Y)))

(event `EnhancedInput|/Game/Blueprints/InputsAdventureMan/Actions/IA_AdventureJump`
  (params (ActionValue :type Boolean) (ElapsedSeconds :type "Float (double-precision)") (TriggeredSeconds :type "Float (double-precision)") (InputAction :type "InputAction Object Reference" :default "/Game/Blueprints/InputsAdventureMan/Actions/IA_AdventureJump.IA_AdventureJump"))
  (:`Started`
    (`self.Jump`))
  (:`Completed`
    (`self.StopJumping`)))

(fn `UserConstructionScript`)