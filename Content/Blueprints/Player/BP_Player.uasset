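; BP_Player is the player character, handling movement, camera look and jumping through Enhanced Input.
; BeginPlay adds the IMC_Player mapping context to the subsystem of player controller 0.
; Movement input follows the right and forward vectors of the full control rotation, while camera input drives controller yaw and pitch.
; Jump starts and stops with the jump action's Started and Completed events.
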(event `self.ReceiveBeginPlay`
  (bind _returnvalue (pcsubsystem `EnhancedInputLocalPlayerSubsystem` (`GameplayStatics.GetPlayerController` 0)))
  (`/Engine/EditorBlueprintResources/StandardMacros.IsValid` _returnvalue
    (:`Is Valid`
      (`EnhancedInputSubsystemInterface.AddMappingContext` _returnvalue "/Game/Blueprints/Inputs/IMC_Player.IMC_Player" 0 (struct)))))

(event `EnhancedInput|/Game/Blueprints/Inputs/Actions/IA_PlayerMovement`
  (params (ActionValue :type "Vector2D Structure") (ElapsedSeconds :type "Float (double-precision)") (TriggeredSeconds :type "Float (double-precision)") (InputAction :type "InputAction Object Reference" :default "/Game/Blueprints/Inputs/Actions/IA_PlayerMovement.IA_PlayerMovement"))
  ;[1 1 1] Input movement
  (:`Triggered`
    (`self.AddMovementInput` (`KismetMathLibrary.GetRightVector` (`self.GetControlRotation`)) ActionValue_X)
    (`self.AddMovementInput` (`KismetMathLibrary.GetForwardVector` (`self.GetControlRotation`)) ActionValue_Y)))

(event `EnhancedInput|/Game/Blueprints/Inputs/Actions/IA_PlayerCamera`
  (params (ActionValue :type "Vector2D Structure") (ElapsedSeconds :type "Float (double-precision)") (TriggeredSeconds :type "Float (double-precision)") (InputAction :type "InputAction Object Reference" :default "/Game/Blueprints/Inputs/Actions/IA_PlayerCamera.IA_PlayerCamera"))
  ;[1 1 1] Input Camera
  (:`Triggered`
    (`self.AddControllerYawInput` ActionValue_X)
    (`self.AddControllerPitchInput` ActionValue_Y)))

(event `EnhancedInput|/Game/Blueprints/Inputs/Actions/IA_PlayerJump`
  (params (ActionValue :type Boolean) (ElapsedSeconds :type "Float (double-precision)") (TriggeredSeconds :type "Float (double-precision)") (InputAction :type "InputAction Object Reference" :default "/Game/Blueprints/Inputs/Actions/IA_PlayerJump.IA_PlayerJump"))
  ;[1 1 1] Input jump
  (:`Started`
    (`self.Jump`))
  (:`Completed`
    (`self.StopJumping`)))

(fn `UserConstructionScript`)